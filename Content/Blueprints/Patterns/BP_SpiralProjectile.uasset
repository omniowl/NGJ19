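; BP_SpiralProjectile is a pattern projectile that moves its Projectile component in an expanding spiral.
; Every tick it lerps amplitude and speed multiplier between min and max values over ExpansionTime, then derives an angle from RotationsPerSecond, that multiplier and time since creation.
; Sine and cosine of the angle give an X/Z offset, added cumulatively to relative location without sweep or delta-time scaling, so motion depends on frame rate.
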(event `self.ReceiveTick`
  (params (DeltaSeconds :type "Float (single-precision)"))
  (bind _returnvalue (`self.GetGameTimeSinceCreation`))
  (bind _amplitude (`self.Amplitude`))
  (bind _returnvalue_2 (`KismetMathLibrary.FClamp` (/ _returnvalue (`self.ExpansionTime`))))
  (set `self.Amplitude` (`KismetMathLibrary.Lerp` (`self.MinAmp`) (`self.MaxAmp`) _returnvalue_2))
  (bind _output_get (set `self.Theta` (* (`KismetMathLibrary.MultiplyByPi` (* (`self.RotationsPerSecond`) (`KismetMathLibrary.Lerp` (`self.MinSpeed`) (`self.MaxSpeed`) _returnvalue_2))) _returnvalue)))
  (`SceneComponent.K2_AddRelativeLocation` (`self.Projectile`) (`KismetMathLibrary.MakeVector` (* (`KismetMathLibrary.Sin` _output_get) _amplitude) 0.0 (* _amplitude (`KismetMathLibrary.Cos` _output_get))) false false))

(fn `UserConstructionScript`
  (`parent.UserConstructionScript`))