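; BP_SineProjectile is a projectile Blueprint that oscillates its Projectile component along the relative Z axis.
; Each Tick advances a Time value scaled by Frequency and adds its sine, scaled by Amplitude, as a relative location offset without sweeping.
; The offset accumulates per frame without DeltaSeconds scaling, so the wave's size depends on frame rate.
; The construction script only calls the parent's.
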(event `self.ReceiveTick`
  (params (DeltaSeconds :type "Float (single-precision)"))
  (bind _output_get (set `self.Time` (+ (`self.Time`) (* DeltaSeconds (`self.Frequency`)))))
  (bind _output_get_2 (set `self.Theta` (`KismetMathLibrary.Sin` _output_get)))
  (`SceneComponent.K2_AddRelativeLocation` (`self.Projectile`) (`KismetMathLibrary.MakeVector` 0.0 0.0 (* _output_get_2 (`self.Amplitude`))) false false))

(fn `UserConstructionScript`
  (`parent.UserConstructionScript`))