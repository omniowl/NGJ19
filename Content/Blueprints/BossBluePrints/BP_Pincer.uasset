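; BP_Pincer is a boss pincer actor that slides along the world X axis to a stop position and back.
; StartPincer runs a timeline that lerps X from the position captured in the construction script, then waits before calling ResetPincer.
; ResetPincer plays a second timeline over the same lerp to return it, then fires the PincerReturned dispatcher.
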(event `StartPincer`
  (bind (_returnvalue_x _returnvalue_y _returnvalue_z) (`KismetMathLibrary.BreakVector` (`self.K2_GetActorLocation`)))
  (bind _startposition_x (`KismetMathLibrary.BreakVector` (`self.StartPosition`)))
  (bind (_direction _pincertime) (`Timeline|MovePincer` :!via `PlayFromStart`)
    (:`Update`
      (`self.K2_SetActorLocation` (`KismetMathLibrary.MakeVector` (`KismetMathLibrary.Lerp` _startposition_x (`self.StopPosition`) _pincertime) _returnvalue_y _returnvalue_z)))
    (:`Finished`
      (`KismetSystemLibrary.Delay` (`self.DelayTime`))
      (`self.ResetPincer`))))

(event `ResetPincer`
  (bind (_returnvalue_x _returnvalue_y _returnvalue_z) (`KismetMathLibrary.BreakVector` (`self.K2_GetActorLocation`)))
  (bind _startposition_x (`KismetMathLibrary.BreakVector` (`self.StartPosition`)))
  (bind (_direction _pincertime) (`Timeline|ReturnPincer` :!via `PlayFromStart`)
    (:`Update`
      (`self.K2_SetActorLocation` (`KismetMathLibrary.MakeVector` (`KismetMathLibrary.Lerp` _startposition_x (`self.StopPosition`) _pincertime) _returnvalue_y _returnvalue_z)))
    (:`Finished`
      (`self.PincerReturned`))))

(fn `UserConstructionScript`
  (set `self.StartPosition` (`self.K2_GetActorLocation`)))