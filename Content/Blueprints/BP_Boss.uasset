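; BP_Boss is a boss enemy that bobs on a timeline between its placed position and an offset along Z.
; Hitbox overlaps deal damage from attacking heavy-player blades or from projectiles, which also build stun, and both fire event dispatchers.
; While unstunned, Tick sets IsAttacking and picks an attack enum, but nothing here executes it or clears either flag.
; The attack picker re-rolls 0–1 per check against bands scaled to 100, so the intended weighting fails.
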(event `self.HitBox.OnComponentBeginOverlap`
  (params (OverlappedComponent :type "PrimitiveComponent Object Reference") (OtherActor :type "Actor Object Reference") (OtherComp :type "PrimitiveComponent Object Reference") (OtherBodyIndex :type Integer) (bFromSweep :type Boolean) (SweepResult :type "HitResult Structure (by ref)"))
  (bind _asbox_collision (cast `BoxComponent` OtherComp)
    (:`then`
      (if (`ActorComponent.ComponentHasTag` _asbox_collision "Blade")
        (bind _asbp_heavy_player (cast `/Game/Blueprints/BP_HeavyPlayer` (`ActorComponent.GetOwner` _asbox_collision)))
        (if (`/Game/Blueprints/BP_HeavyPlayer.IsAttacking?` _asbp_heavy_player)
          (`self.TakeDamage` false))
        (else
          (bind _asbp_projectile (cast `/Game/Blueprints/BP_Projectile` OtherActor :!label _label))
          (`self.TakeDamage` true)
          (`self.K2_DestroyActor` _asbp_projectile))))
    (:`CastFailed`
      (goto _label))))

(event `TakeDamage`
  (params (`IsShuriken?` :type Boolean))
  (set `self.CurrentHealth` (- (`self.CurrentHealth`) 10.0))
  (`self.BossTookDamage`)
  (if `IsShuriken?`
    (set `self.CurrentStun` (+ (`self.CurrentStun`) 1))
    (if (>= (`self.CurrentStun`) (`self.TargetStun`))
      (set `self.CurrentStun` 0)
      (set `self.IsStunned` true))
    (`self.BossTookStunDamage`)))

(event `VisualizeDamage`)

(event `self.ReceiveBeginPlay`
  (bind (_direction _floatingdelta) (`Timeline|FloatingUpAndDown`)
    (:`Update`
      (`self.K2_SetActorLocation` (`KismetMathLibrary.VLerp` (`self.StartPosition`) (`self.EndPosition`) _floatingdelta)))))

(event `self.ReceiveTick`
  (params (DeltaSeconds :type "Float (single-precision)"))
  (if (`self.IsStunned`)
    _
    (elif (not (`self.IsAttacking`))
      (set `self.IsAttacking` true)
      (`self.PickRandomAttack`))))

(fn `PickRandomAttack`
  (returns (NextAttack :type "/Game/Blueprints/Enums/BossAttack Enum"))
  (locals (ResultAttack :type "/Game/Blueprints/Enums/BossAttack Enum"))
  (bind _returnvalue (`KismetMathLibrary.RandomFloatInRange` 0.0 1.0))
  (if (`self.CheckInbetweenRange` _returnvalue 0.0 10.0)
    (set `local.ResultAttack` "NewEnumerator3")
    (return (`local.ResultAttack`))
    (elif (`self.CheckInbetweenRange` _returnvalue 11.0 35.0)
      (set `local.ResultAttack` "NewEnumerator0")
      (return (`local.ResultAttack`))
      (elif (`self.CheckInbetweenRange` _returnvalue 36.0 75.0)
        (set `local.ResultAttack` "NewEnumerator1")
        (return (`local.ResultAttack`))
        (elif (`self.CheckInbetweenRange` _returnvalue 76.0 100.0)
          (set `local.ResultAttack` "NewEnumerator2")
          (return (`local.ResultAttack`)))))))

(fn `UserConstructionScript`
  (bind _output_get (set `self.StartPosition` (`self.K2_GetActorLocation`)))
  (set `self.EndPosition` (`KismetMathLibrary.MakeVector` (.x _output_get) (.y _output_get) (- (.z _output_get) (`self.FloatOffset`)))))