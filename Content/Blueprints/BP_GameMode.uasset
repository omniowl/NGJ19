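; Game mode for a local two-player match that gives each player a different character.
; BeginPlay creates local players for controller IDs 0 and 1.
; The SpawnDefaultPawnFor override uses a Players counter to spawn a light character first and a heavy one second at the given start spot.
; It possesses each, forces its facing direction and sets its damage, also setting the heavy character's jump count.
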(event `self.ReceiveBeginPlay`
  (`GameplayStatics.CreatePlayer` 0)
  (`GameplayStatics.CreatePlayer` 1))

(fn `SpawnDefaultPawnFor`
  (params (NewPlayer :type "Controller Object Reference") (StartSpot :type "Actor Object Reference"))
  (returns (ReturnValue :type "Pawn Object Reference"))
  (bind _returnvalue (`self.GetTransform` StartSpot))
  (switch `int` (`self.Players`)
    (:`0`
      (bind _returnvalue_2 (`|SpawnActorFromClass` "/Game/Blueprints/BP_LightPlayer.BP_LightPlayer_C" _returnvalue "Undefined" "OverrideRootScale" NewPlayer null))
      (`Controller.Possess` NewPlayer _returnvalue_2)
      (set `/Game/Blueprints/BP_LightPlayer.Direction` "NewEnumerator1" _returnvalue_2)
      (`/Game/Blueprints/BP_LightPlayer.ForceRotation` _returnvalue_2)
      (set `/Game/Blueprints/BP_LightPlayer.Damage` 10.0 _returnvalue_2)
      (set `self.Players` 1)
      (return _returnvalue_2))
    (:`1`
      (bind _returnvalue_3 (`|SpawnActorFromClass` "/Game/Blueprints/BP_HeavyPlayer.BP_HeavyPlayer_C" _returnvalue "Undefined" "OverrideRootScale" NewPlayer null))
      (`Controller.Possess` NewPlayer _returnvalue_3)
      (set `/Game/Blueprints/BP_HeavyPlayer.Direction` "NewEnumerator0" _returnvalue_3)
      (`/Game/Blueprints/BP_HeavyPlayer.ForceRotation` _returnvalue_3)
      (set `/Game/Blueprints/BP_HeavyPlayer.Damage` 20.0 _returnvalue_3)
      (set `/Game/Blueprints/BP_HeavyPlayer.MaxJumpCount` 1 _returnvalue_3)
      (return _returnvalue_3))))

(fn `UserConstructionScript`)